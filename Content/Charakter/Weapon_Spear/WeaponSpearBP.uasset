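; Spear weapon actor that damages DinoCritter enemies it overlaps while the player character is attacking.
; On overlap it reads IsAttacking from player 0's CharakterBP rather than from an owner reference.
; Only actors whose class is exactly DinoCritter lose a fixed amount of Health, set directly without the damage system.
; A critter is destroyed once its Health drops below the player's MimimumHealth value.
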(event EventActorBeginOverlap
  (params (OtherActor :type Actor%20Object%20Reference))
  (bind _ascharakter_bp (Utilities|Casting|CastToCharakterBP (Game|GetPlayerCharacter 0)))
  (if (Variables|/Game/Charakter/CharakterBP.CharakterBP_C|GetisAttacking _ascharakter_bp)
    (if (== (Utilities|GetClass OtherActor) "/Game/Dinosaurs/Character/DinoCritter.DinoCritter_C")
      (bind _asdino_critter (Utilities|Casting|CastToDinoCritter OtherActor))
      (bind _output_get (Variables|/Game/Dinosaurs/Character/DinoCritter.DinoCritter_C|SetHealth _asdino_critter (- (Variables|/Game/Dinosaurs/Character/DinoCritter.DinoCritter_C|GetHealth _asdino_critter) 5e+01)))
      (if (< _output_get (Variables|/Game/Charakter/CharakterBP.CharakterBP_C|GetMimimumHealth _ascharakter_bp))
        (Actor|DestroyActor OtherActor)))))

(fn ConstructionScript)