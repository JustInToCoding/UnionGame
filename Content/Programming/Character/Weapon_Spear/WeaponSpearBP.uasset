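; Spear weapon actor that damages AI creatures it overlaps during the player's attack.
; On begin overlap, it checks that player character 0's IsAttackingTimer is at least zero.
; It then matches the other actor's exact class against AICritter, AISmallEnemy and AIBaby in turn, passing Damage to DamageCritter for critters or DamageEnemy for the other two.
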(event EventActorBeginOverlap
  (params (OtherActor :type Actor%20Object%20Reference))
  (bind _returnvalue (Utilities|GetClass OtherActor))
  (bind _damage (Variables|Default|GetDamage))
  (bind _asmy_character (Utilities|Casting|CastToMyCharacter (Game|GetPlayerCharacter 0)))
  (if (>= (Variables|/Game/Programming/Character/MyCharacter.MyCharacter_C|GetisAttackingTimer _asmy_character) 0.0)
    (if (== _returnvalue "/Game/Programming/Dinosaurs/Critter/AICritter.AICritter_C")
      (bind _asaicritter (Utilities|Casting|CastToAICritter OtherActor))
      (Default|DamageCritter _asaicritter _damage)
      (elif (== _returnvalue "/Game/Programming/Dinosaurs/Small/AISmallEnemy.AISmallEnemy_C")
        (bind _asaismall_enemy (Utilities|Casting|CastToAISmallEnemy OtherActor))
        (Default|DamageEnemy _asaismall_enemy _damage)
        (elif (== _returnvalue "/Game/Programming/Dinosaurs/Small/AIBaby.AIBaby_C")
          (bind _asaibaby (Utilities|Casting|CastToAIBaby OtherActor))
          (Default|DamageEnemy _asaibaby _damage))))))

(fn ConstructionScript)