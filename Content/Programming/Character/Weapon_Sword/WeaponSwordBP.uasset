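; Sword weapon Blueprint that damages AI creatures it begins overlapping while the player is mid-attack.
; Hits count only while the player character's attack timer is within a short window.
; An exact class check routes the Damage value to the matching critter, small enemy or baby damage function, then plays a flesh impact sound at the sword's location.
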(event EventActorBeginOverlap
  (params (OtherActor :type Actor%20Object%20Reference))
  (bind _returnvalue (Utilities|GetClass OtherActor))
  (bind _damage (Variables|Default|GetDamage))
  (bind _asmy_character (Utilities|Casting|CastToMyCharacter (Game|GetPlayerCharacter 0)))
  (if (and (>= (Variables|/Game/Programming/Character/MyCharacter.MyCharacter_C|GetisAttackingTimer _asmy_character) 0.0) (< (Variables|/Game/Programming/Character/MyCharacter.MyCharacter_C|GetisAttackingTimer _asmy_character) 0.5))
    (if (== _returnvalue "/Game/Programming/Dinosaurs/Critter/AICritter.AICritter_C")
      (bind _asaicritter (Utilities|Casting|CastToAICritter OtherActor))
      (Default|DamageCritter _asaicritter _damage)
      (Audio|PlaySoundatLocation "/Game/Programming/Character/Sounds/ImpactFlesh/ImpactFlesh.ImpactFlesh" (Transformation|GetActorLocation) :!label _label)
      (elif (== _returnvalue "/Game/Programming/Dinosaurs/Small/AISmallEnemy.AISmallEnemy_C")
        (bind _asaismall_enemy (Utilities|Casting|CastToAISmallEnemy OtherActor))
        (Default|DamageEnemy _asaismall_enemy _damage)
        (goto _label)
        (elif (== _returnvalue "/Game/Programming/Dinosaurs/Small/AIBaby.AIBaby_C")
          (bind _asaibaby (Utilities|Casting|CastToAIBaby OtherActor))
          (Default|DamageEnemy _asaibaby _damage)
          (goto _label))))))

(fn ConstructionScript)