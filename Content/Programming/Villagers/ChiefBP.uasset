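; ChiefBP holds the health and stamina logic for the Chief and shows both values on the HUD.
; Regen functions add per-call amounts, with the stamina rate switching between idle and moving values based on velocity; no caller appears here.
; Stamina is clamped between zero and its maximum, while health regen runs only between those limits and can overshoot the maximum.
; UpdateHUD pushes both values to player 0's MyHUD and prints health.
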(fn ConstructionScript)

(fn HealthRegen
  (if (and (< (Variables|Health|GetHealth) (Variables|Health|GetMaxHealth)) (> (Variables|Health|GetHealth) 0.0))
    (Variables|Health|SetHealth (+ (Variables|Health|GetHealth) (Variables|Health|GetHealthRegenPerSecond)))
    (CallFunction|UpdateHUD)))

(fn StaminaRegen
  (if (Math|Vector|Equal(Vector) (Transformation|GetVelocity) "0, 0, 0" 0.0001)
    (Variables|Stamina|SetStaminaRegenPerSecond (Variables|Stamina|GetStaminaRegenIdle))
    (else
      (Variables|Stamina|SetStaminaRegenPerSecond (Variables|Stamina|GetStaminaRegenMoving))))
  (if (< (+ (Variables|Stamina|GetStamina) (Variables|Stamina|GetStaminaRegenPerSecond)) 0.0)
    (Variables|Stamina|SetStamina 0.0)
    (else
      (if (> (+ (Variables|Stamina|GetStamina) (Variables|Stamina|GetStaminaRegenPerSecond)) (Variables|Stamina|GetMaxStamina))
        (Variables|Stamina|SetStamina (Variables|Stamina|GetMaxStamina))
        (else
          (Variables|Stamina|SetStamina (+ (Variables|Stamina|GetStamina) (Variables|Stamina|GetStaminaRegenPerSecond)))))
      (CallFunction|UpdateHUD))))

(fn ReduceStamina
  (params (Amount :type Float%20%28single-precision%29 :default 0.0))
  (if (< (- (Variables|Stamina|GetStamina) Amount) 0.0)
    (Variables|Stamina|SetStamina 0.0)
    (else
      (Variables|Stamina|SetStamina (- (Variables|Stamina|GetStamina) Amount))))
  (CallFunction|UpdateHUD))

(fn UpdateHUD
  (bind _health (Variables|Health|GetHealth))
  (bind _asmy_hud (Utilities|Casting|CastToMyHUD (HUD|GetHUD (Game|GetPlayerController 0))))
  (Class|MyHUD|SetHealth _asmy_hud _health)
  (Development|PrintText (Utilities|Text|ToText(Float) _health "HalfToEven"))
  (Class|MyHUD|SetStamina _asmy_hud (Variables|Stamina|GetStamina)))