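; FemaleBP is a villager that wanders on its own between AreaVillager actors placed in the level.
; BeginPlay gathers those areas and picks a random starting area and destination.
; Tick runs two randomized countdowns: a long travel timer that switches areas and a short roam timer that picks a new random point around the current area.
; On ticks where neither timer expires, it reissues AIMoveTo toward the stored destination.
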(event EventTick
  (params (DeltaSeconds :type Float%20%28single-precision%29))
  (bind _myareas (Variables|Default|GetMyAreas))
  (bind _output_get (Variables|Default|SetTravelTime (- (Variables|Default|GetTravelTime) DeltaSeconds)))
  (if (<= _output_get 0.0)
    (bind _output_get_2 (Variables|Default|SetMyArea (Utilities|Array|Get(acopy) _myareas (Math|Random|RandomInteger (Utilities|Array|Length _myareas)))))
    (Variables|Default|SetMoveTo (Class|NavigationSystem|GetRandomPointinRadius (Transformation|GetActorLocation _output_get_2) 5e+02))
    (Variables|Default|SetTravelTime (Math|Random|RandomFloatinRange 2e+01 4e+01))
    (Variables|Default|SetRoamTime (Math|Random|RandomFloatinRange 3.0 1e+01))
    (else
      (bind _output_get_3 (Variables|Default|SetRoamTime (- (Variables|Default|GetRoamTime) DeltaSeconds)))
      (if (<= _output_get_3 0.0)
        (Variables|Default|SetMoveTo (Class|NavigationSystem|GetRandomPointinRadius (Transformation|GetActorLocation (Variables|Default|GetMyArea)) 5e+02))
        (Variables|Default|SetRoamTime (Math|Random|RandomFloatinRange 3.0 1e+01))
        (else
          (AI|AIMoveTo self (Variables|Default|GetMoveTo) 0 5.0 false))))))

(event EventBeginPlay
  (bind _outactors (Actor|GetAllActorsOfClass "/Game/ProgrammingPlaceable/AreaVillager.AreaVillager_C"))
  (bind _output_get (Variables|Default|SetMyAreas _outactors))
  (Variables|Default|SetMyArea (Utilities|Array|Get(acopy) _output_get (Math|Random|RandomInteger (Utilities|Array|Length _output_get))))
  (Variables|Default|SetMoveTo (Transformation|GetActorLocation (Utilities|Array|Get(acopy) _output_get (Math|Random|RandomInteger (Utilities|Array|Length _output_get)))))
  (Variables|Default|SetTravelTime (Math|Random|RandomFloatinRange 2e+01 4e+01))
  (Variables|Default|SetRoamTime (Math|Random|RandomFloatinRange 3.0 1e+01)))

(fn ConstructionScript)