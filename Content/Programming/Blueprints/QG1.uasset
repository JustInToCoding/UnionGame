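; Quest giver actor for quest "q01" that shows its dialogue as printed, color-coded messages.
; An outer trigger prints the opening message while the quest is startable; an inner trigger enables input.
; E steps through the start conversation, then triggers the quest and spawns Dinos at the placed actors' transforms.
; In later states E prints the current message, triggering the quest again when completed; F prints the state.
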(event OnComponentBeginOverlap(Inner)
  (params (OtherActor :type Actor%20Object%20Reference) (OtherComp :type Primitive%20Component%20Object%20Reference) (OtherBodyIndex :type Integer) (bFromSweep :type Boolean) (SweepResult :type Hit%20Result%20Structure%20%28by%20ref%29))
  (Input|EnableInput (Game|GetPlayerController 0)))

(event OnComponentBeginOverlap(Outer)
  (params (OtherActor :type Actor%20Object%20Reference) (OtherComp :type Primitive%20Component%20Object%20Reference) (OtherBodyIndex :type Integer) (bFromSweep :type Boolean) (SweepResult :type Hit%20Result%20Structure%20%28by%20ref%29))
  (bind _returnvalue (Class|QuestManager|GetQuest "q01"))
  (switch Utilities|FlowControl|Switch|SwitchonEQuestStateEnum (Class|BlueprintQuest|GetCurrentState _returnvalue)
    (:VE_Startable
      (Development|PrintString (Utilities|Array|Get(acopy) (Class|BlueprintQuest|GetMessages _returnvalue))))))

(event OnComponentEndOverlap(Inner)
  (params (OtherActor :type Actor%20Object%20Reference) (OtherComp :type Primitive%20Component%20Object%20Reference) (OtherBodyIndex :type Integer))
  (Input|DisableInput (Game|GetPlayerController 0)))

(event Input|KeyboardEvents|E
  (:Pressed
    (CallFunction|UpdateQuestVariables)
    (CallFunction|UpdateTextColor (Variables|Default|GetmsgCount) (Variables|Default|GetcurrentState))
    (switch Utilities|FlowControl|Switch|SwitchonEQuestStateEnum (Variables|Default|GetcurrentState)
      (:VE_Startable
        (CallFunction|StartConversation))
      (:VE_Running
        (Development|PrintString (Utilities|Array|Get(acopy) (Variables|Default|GetcurrentMessages)) true true (Variables|Default|GetcurrentColor) :!label _label)
        (switch Utilities|FlowControl|Switch|SwitchonEQuestStateEnum (Variables|Default|GetcurrentState)
          (:VE_Completed
            (Class|BlueprintQuest|Trigger (Class|QuestManager|GetQuest "q01")))))
      (:VE_Completed
        (goto _label))
      (:VE_ClosedSuccessful
        (goto _label)))))

(event Input|KeyboardEvents|F
  (:Pressed
    (CallFunction|UpdateQuestVariables)
    (Development|PrintString (Utilities|String|ToString(Byte) (Variables|Default|GetcurrentState)))))

(fn ConstructionScript)

(fn UpdateTextColor
  (params (msgID :type Integer :default 0) (state :type EQuestStateEnum%20Enum :default "VE_NotSet"))
  (switch Utilities|FlowControl|Switch|SwitchonEQuestStateEnum state
    (:VE_Startable
      (if (== msgID 1)
        (Variables|Default|SetcurrentColor "(R=0.994000,G=0.000000,B=0.000000,A=1.000000)")
        (else
          (Variables|Default|SetcurrentColor "(R=0.000000,G=0.000000,B=0.994000,A=1.000000)" :!label _label))))
    (:VE_Running
      (goto _label))
    (:VE_Completed
      (goto _label))
    (:VE_ClosedSuccessful
      (goto _label))))

(fn UpdateQuestVariables
  (bind _returnvalue (Class|QuestManager|GetQuest "q01"))
  (Variables|Default|SetcurrentMessages (Class|BlueprintQuest|GetMessages _returnvalue))
  (Variables|Default|SetcurrentState (Class|BlueprintQuest|GetCurrentState _returnvalue)))

(fn StartConversation
  (Development|PrintString (Utilities|Array|Get(acopy) (Variables|Default|GetcurrentMessages) (Variables|Default|GetmsgCount)) true true (Variables|Default|GetcurrentColor))
  (bind _output_get (Variables|Default|SetmsgCount (+ (Variables|Default|GetmsgCount) 1)))
  (if (>= _output_get (Utilities|Array|Length (Variables|Default|GetcurrentMessages)))
    (Class|BlueprintQuest|Trigger (Class|QuestManager|GetQuest "q01"))
    (for _array_element (Variables|Default|GetDinos)
      (Game|SpawnActorfromClass "/Game/Programming/Blueprints/Dino.Dino_C" (Transformation|GetActorTransform _array_element) false 0)
      (Variables|Default|SetmsgCount 1))))