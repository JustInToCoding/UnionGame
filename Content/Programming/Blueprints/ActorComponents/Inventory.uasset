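; Inventory actor component that exercises the inventory system through debug events.
; DisplayInventory loops over the current inventory from a singleton instance, looks up each item's name by Id and prints it with its amount.
; AddToInventory and RemoveFromInventory apply hardcoded test item changes to that same instance and print the result, with removal reporting success or failure.
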(event Custom|DisplayInventory
  (for _array_element (Class|Inventory|GetCurrentInventory (Class|Inventory|GetInstance))
    (Development|PrintString (Utilities|String|Append (Utilities|String|Append (Class|BlueprintItem|GetName (Class|ItemManager|GetItem (Class|ItemManager|GetInstance) (.id (Utilities|Struct|BreakEntry _array_element)))) " ") (Utilities|String|ToString(Integer) (.amount (Utilities|Struct|BreakEntry _array_element)))))))

(event Custom|AddToInventory
  (Class|Inventory|AddtoInventory (Class|Inventory|GetInstance) "I01" 2)
  (Development|PrintString "Stuff added"))

(event Custom|RemoveFromInventory
  (bind _returnvalue (Class|Inventory|RemovefromInventory (Class|Inventory|GetInstance) "I01" 3))
  (if _returnvalue
    (Development|PrintString "Removed from inventory")
    (else
      (Development|PrintString "Could not remove from inventory"))))

(event EventTick
  (params (DeltaSeconds :type Float%20%28single-precision%29)))

(event EventInitializeComponent)