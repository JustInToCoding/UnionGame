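; CraftingManager is an actor component Blueprint that exposes debug-style events for listing, checking and crafting items.
; Each event delegates to a singleton reached through GetInstance, which supplies the craftable list and performs the CanCraft and CraftItem calls.
; Results go only to Print String: ListCraftable prints every entry whether craftable or not, while CraftItem and CanCraft report success or failure for a given ID.
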(event Custom|ListCraftable
  (bind _returnvalue (Class|CraftingManager|GetInstance))
  (bind _returnvalue_2 (Class|CraftingManager|GetAllCraftable _returnvalue))
  (for _array_element _returnvalue_2
    (bind _returnvalue_3 (Class|CraftingManager|CanCraft _returnvalue _array_element))
    (if _returnvalue_3
      (Development|PrintString _array_element)
      (else
        (Development|PrintString _array_element true true "(R=1.000000,G=0.059521,B=0.088175,A=1.000000)")))))

(event Custom|CraftItem
  (params (ID :type String))
  (bind _returnvalue (Class|CraftingManager|CraftItem (Class|CraftingManager|GetInstance) ID))
  (if _returnvalue
    (Development|PrintString "Item crafted")
    (else
      (Development|PrintString "Failed to craft item"))))

(event Custom|CanCraft
  (params (ID :type String))
  (bind _returnvalue (Class|CraftingManager|CanCraft (Class|CraftingManager|GetInstance) ID))
  (if _returnvalue
    (Development|PrintString "Item can be crafted")
    (else
      (Development|PrintString "Item can't be crafted"))))

(event EventTick
  (params (DeltaSeconds :type Float%20%28single-precision%29)))

(event EventInitializeComponent)