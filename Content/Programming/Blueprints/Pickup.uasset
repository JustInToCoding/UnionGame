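; Interactable pickup actor that can grant an item to the inventory when E is pressed nearby.
; Capsule overlaps filtered by the TriggerCast macro enable and disable input from player 0, limiting the key to that range.
; On press, the Pickup flag gates AddToInventory, which passes the item ID and a random min-to-max amount to GetInstance's inventory.
; The actor is destroyed whether or not the flag is set.
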(event OnComponentBeginOverlap(Capsule)
  (params (OtherActor :type Actor%20Object%20Reference) (OtherComp :type Primitive%20Component%20Object%20Reference) (OtherBodyIndex :type Integer) (bFromSweep :type Boolean) (SweepResult :type Hit%20Result%20Structure%20%28by%20ref%29))
  (Utilities|TriggerCast OtherActor
    (:Successful
      (Input|EnableInput (Game|GetPlayerController 0)))))

(event OnComponentEndOverlap(Capsule)
  (params (OtherActor :type Actor%20Object%20Reference) (OtherComp :type Primitive%20Component%20Object%20Reference) (OtherBodyIndex :type Integer))
  (Utilities|TriggerCast OtherActor
    (:Successful
      (Input|DisableInput (Game|GetPlayerController 0)))))

(event Input|KeyboardEvents|E
  (:Pressed
    (if (Variables|Default|Getpickup)
      (Utilities|AddtoInventory
        (:Out
          _)))
    (Actor|DestroyActor)))

(fn ConstructionScript)