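; Dino combat Blueprint that tracks which pawns the dinosaur can currently see; it contains only perception logic, with no attacks yet.
; PawnSensing sightings add pawns uniquely to NoticedPawns.
; Since PawnSensing gives no lost-sight event here, a looping half-second timer rechecks each entry against view cone, sight radius and controller line of sight.
; Failures call LostLOS, which removes the pawn mid-loop; both transitions print debug text.
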(event OnSeePawn(PawnSensing)
  (params (Pawn :type Pawn%20Object%20Reference))
  ;[1 1 1] Seeing Pawns
  (Utilities|Array|AddUnique (Variables|Default|GetNoticedPawns) Pawn)
  (Development|PrintText (Utilities|Text|FormatText "Saw Pawn {Pawn}" (Utilities|Text|ToText(String) (Utilities|String|ToString(Object) Pawn)))))

(event Custom|Lost%20LOS
  (params (Pawn :type Pawn%20Object%20Reference))
  ;[1 1 1] Lost LoS With Pawns
  (Utilities|Array|RemoveItem (Variables|Default|GetNoticedPawns) Pawn)
  (Development|PrintText (Utilities|Text|FormatText "Lost Pawn {Pawn}" (Utilities|Text|ToText(String) (Utilities|String|ToString(Object) Pawn))) true true "(R=1.000000,G=0.000000,B=0.018721,A=1.000000)"))

(event Custom|LOS%20Check
  (bind _pawnsensing (Variables|Default|GetPawnSensing))
  ;[1 1 1] Check if noticed pawns are still in line of sight
  (for _array_element (Variables|Default|GetNoticedPawns)
    (if (Math|Boolean|ORBoolean (< (Math|Vector|DotProduct (Transformation|GetActorForwardVector) (- (Transformation|GetActorLocation _array_element) (Transformation|GetActorLocation))) (Class|PawnSensingComponent|GetPeripheralVisionCosine _pawnsensing)) (> (Math|Vector|VectorLength (- (Transformation|GetActorLocation _array_element) (Transformation|GetActorLocation))) (Variables|/Script/AIModule.PawnSensingComponent|GetSightRadius _pawnsensing)) (not (Controller|LineOfSightTo (Pawn|GetController) _array_element "0, 0, 0" false)))
      (CallFunction|LostLOS _array_element))))

(event EventBeginPlay
  (Utilities|Time|SetTimerbyEvent (delegate Custom|LOS%20Check) 0.5 true))

(event EventActorBeginOverlap
  (params (OtherActor :type Actor%20Object%20Reference)))

(event EventTick
  (params (DeltaSeconds :type Float%20%28single-precision%29)))

(fn ConstructionScript)